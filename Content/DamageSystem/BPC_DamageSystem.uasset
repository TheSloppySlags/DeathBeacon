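; Damage system Blueprint component that tracks health, death, invincibility and blocking, and handles healing and incoming damage.
; Heal clamps Health to MaxHealth while alive, and TakeDamage routes a DamageInfo through the CanBeDamaged macro to block, damage or ignore it.
; Dispatchers announce blocks, death and damage responses, the latter only for interruptible or force-interrupting hits.
; TakeDamage returns true only after death or a damage response is broadcast.
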(event EventBeginPlay)

(event EventTick
  (params (DeltaSeconds :type Float%20%28single-precision%29)))

(fn Heal
  (params (Amount :type Float%20%28double-precision%29))
  (if (not (Variables|Default|GetDead?))
    (Variables|Default|SetHealth (Math|Float|Clamp(Float) (+ Amount (Variables|Default|GetHealth)) 0.0 (Variables|Default|GetMaxHealth)))
    (return 0.0)))

(fn TakeDamage
  (params (DamageInfo :type BP%20Damage%20Info%20Structure))
  (bind (_amount _damagetype _damageresponse _shoulddamageinvincible_ _canbeblocked_ _shouldforceinterrupt) (Utilities|Struct|BreakBP_DamageInfo DamageInfo))
  (Utilities|CanbeDamaged _shoulddamageinvincible_ _canbeblocked_
    (:BlockDamage
      (Default|CallOnBlocked)
      (return false))
    (:DoDamage
      (bind _output_get (Variables|Default|SetHealth (- (Variables|Default|GetHealth) _amount)))
      (if (<= _output_get 0.0)
        (Variables|Default|SetDead? true)
        (Default|CallOnDeath)
        (return true)
        (elif (or (Variables|Default|GetIsInterruptible?) _shouldforceinterrupt)
          (Default|CallOnDamageResponse _damageresponse)
          (return true))))
    (:NoDamage
      (return false))))